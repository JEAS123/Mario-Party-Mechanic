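; Board-game character pawn that takes a dice turn, moving along linked spaces and gaining or losing coins in Mario Party style.
; RollDice blends the camera to the pawn and rolls moves; MoveToSpace repeats AIMoveTo along each first NextSpace link until none remain.
; EndTurn applies the space type: Blue adds coins, Red subtracts, Event randomly changes coins or starts bonus movement.
; Turn-ended and coin-collected dispatchers then fire, without waiting for bonus movement.
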(event `RollDice`
  (`PlayerController.SetViewTargetWithBlend` (`GameplayStatics.GetPlayerController` 0) self 1.5 "VTBlend_Linear" 0.0 false)
  (set `self.MovesRemaining` (`KismetMathLibrary.RandomIntegerInRange` 1 10))
  (`KismetSystemLibrary.Delay` 2.0)
  (`self.MoveToSpace` (`self.CurrentSpace`)))

(event `MoveToSpace`
  (params (CurrentSpace :type "/Game/BP_BoardSpace Object Reference"))
  (bind _output (`|GetArrayItem` (`/Game/BP_BoardSpace.NextSpace` CurrentSpace)))
  (set `self.CurrentSpace` _output)
  (`|AIMoveTo` self (0.0 0.0 0.0) _output
    (:`OnSuccess`
      (bind _result (`/Engine/EditorBlueprintResources/StandardMacros.DecrementInt` (`self.MovesRemaining`))
        (:`  `
          (if (> _result 0)
            (`self.MoveToSpace` (`self.CurrentSpace`))
            (else
              (`self.EndTurn`))))))))

(event `EndTurn`
  (`KismetSystemLibrary.Delay` 3.0)
  (`|ExecutionSequence`
    (:`then_0`
      (switch `/Game/EN_SpaceType` (`/Game/BP_BoardSpace.SpaceType` (`self.CurrentSpace`))
        (:`NewEnumerator0`
          (`self.AddCoins` 3))
        (:`NewEnumerator1`
          (`self.AddCoins` -3))
        (:`NewEnumerator2`
          (`self.EventSpace`))))
    (:`then_1`
      (`self.OnTurnEnded`)
      (`self.OnCoinCollected`))))

(fn `AddCoins`
  (params (Number :type Integer))
  (set `self.Coins` (+ (`self.Coins`) Number)))

(fn `EventSpace`
  (set `self.EventDetermine` (`KismetMathLibrary.RandomIntegerInRange` 0 2))
  (if (== (`self.EventDetermine`) 0)
    (`self.AddCoins` (`KismetMathLibrary.RandomIntegerInRange` 3 20))
    (`KismetSystemLibrary.PrintString` "Lucky; Gain Coins")
    (elif (== (`self.EventDetermine`) 1)
      (`self.AddCoins` (`KismetMathLibrary.RandomIntegerInRange` -30 -3))
      (`KismetSystemLibrary.PrintString` "Unlcuky; Lost Coins")
      (elif (== (`self.EventDetermine`) 2)
        (`PlayerController.SetViewTargetWithBlend` (`GameplayStatics.GetPlayerController` 0) self 1.5 "VTBlend_Linear" 0.0 false)
        (set `self.RollEventDetermine` (`KismetMathLibrary.RandomIntegerInRange` 0 3))
        (if (== (`self.RollEventDetermine`) 0)
          (set `self.MovesRemaining` (`KismetMathLibrary.RandomIntegerInRange` 1 3))
          (`self.MoveToSpace` (`self.CurrentSpace`))
          (`KismetSystemLibrary.PrintString` "Creepy Dice")
          (elif (== (`self.RollEventDetermine`) 1)
            (set `self.MovesRemaining` (`KismetMathLibrary.RandomIntegerInRange` 2 20))
            (`self.MoveToSpace` (`self.CurrentSpace`))
            (`KismetSystemLibrary.PrintString` "Double Dice")
            (elif (== (`self.RollEventDetermine`) 2)
              (set `self.MovesRemaining` (`KismetMathLibrary.RandomIntegerInRange` 3 30))
              (`self.MoveToSpace` (`self.CurrentSpace`))
              (`KismetSystemLibrary.PrintString` "Triple Dice")
              (else
                (set `self.MovesRemaining` 5)
                (`self.MoveToSpace` (`self.CurrentSpace`))
                (`KismetSystemLibrary.PrintString` "Mushroom")))))))))

(fn `UserConstructionScript`)