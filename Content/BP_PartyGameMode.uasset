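; Party game mode that runs repeating rounds in which each BP_Character takes one dice-roll turn.
; BeginPlay gathers all characters as the turn order, starts the first round and shows WBP_HUD.
; Each round copies that order into a queue, calling RollDice on the front character and removing it when its OnTurnEnded fires.
; An empty queue decrements Rounds and starts another round after a delay, with no end condition.
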(event `self.ReceiveBeginPlay`
  ; Initiates "Rounds" that consists of one turn for each Player
  (bind _outactors (`GameplayStatics.GetAllActorsOfClass` "/Game/BP_Character.BP_Character_C"))
  (set `self.TurnOrder` _outactors)
  (`self.InitiateRound`)
  (bind _returnvalue (`|CreateWidget` "/Game/UI/WBP_HUD.WBP_HUD_C"))
  (`UserWidget.AddToViewport` _returnvalue 0))

(event `StartTurn`
  (bind _output (`|GetArrayItem` (`self.RoundOrder`)))
  ; After the Round is initiated, it initiates each Player's Turn within the Round
  (`KismetSystemLibrary.Delay` 2.0)
  (`/Game/BP_Character.RollDice` _output)
  (add `/Game/BP_Character.OnTurnEnded` _output (delegate `NextTurn`)))

(event `InitiateRound`
  ; After the Round is initiated, it initiates each Player's Turn within the Round
  (set `self.RoundOrder` (`self.TurnOrder`))
  (`self.StartTurn`))

(event `NextTurn`
  ; After a Turn is completed, the Round's status is checked. If no more turn remain, it switches to the next round.
  (`KismetArrayLibrary.Array_Remove` (`self.RoundOrder`))
  (if (`KismetArrayLibrary.Array_IsEmpty` (`self.RoundOrder`))
    (`self.EndRound`)
    (else
      (`self.StartTurn`))))

(event `EndRound`
  ; After a Turn is completed, the Round's status is checked. If no more turn remain, it switches to the next round.
  (`/Engine/EditorBlueprintResources/StandardMacros.DecrementInt` (`self.Rounds`)
    (:`  `
      (`KismetSystemLibrary.Delay` 3.0)
      (`self.InitiateRound`))))

(fn `UserConstructionScript`)